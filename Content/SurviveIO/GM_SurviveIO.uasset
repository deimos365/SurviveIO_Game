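; Game mode for SurviveIO that runs a timed survival round, starting all spawners on BeginPlay.
; Binds each spawned enemy's HealthComponent death to add score in GS_SurviveIO, and binds the player pawn's death when spawning it.
; Timer expiry stops spawners, player and enemies; game over stops spawners and clears the timer.
; Both endings show WBP_ResultScreen with the high-score flag, though victory also passes IsVictory as false.
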(event `self.ReceiveBeginPlay`
  (bind _outactors (`GameplayStatics.GetAllActorsOfClass` "/Game/Enemy/BP_Spawner.BP_Spawner_C"))
  (for _array_element _outactors
    (`/Game/Enemy/BP_Spawner.OnGameStart` _array_element)
    (add `/Game/Enemy/BP_Spawner.OnEnemySpawn` _array_element (delegate `OnEnemySpawn`)))
  (`self.StartVictoryTimer`)
  (`WidgetBlueprintLibrary.SetInputMode_GameOnly` (`GameplayStatics.GetPlayerController` 0)))

(event `OnEnemySpawn`
  (params (SpawnedActor :type "Actor Object Reference"))
  (add `/Game/Health/HealthComponent.OnDeath` (`self.GetComponentByClass` SpawnedActor "/Game/Health/HealthComponent.HealthComponent_C") (delegate `OnEnemyDeath`)))

(event `OnEnemyDeath`
  (bind _asgs_survive_io (cast `/Game/SurviveIO/GS_SurviveIO` (`GameplayStatics.GetGameState`)))
  (`/Game/SurviveIO/GS_SurviveIO.AddScore` _asgs_survive_io 20.0))

(event `OnPlayerDeath`
  (`self.OnGameOver`))

(event `OnGameOver`
  (`self.ShowResult` false)
  (`KismetSystemLibrary.K2_ClearAndInvalidateTimerHandle` (`self.VictoryTimerHandle`))
  (`self.StopSpawners`))

(event `StartVictoryTimer`
  (bind _returnvalue (`KismetSystemLibrary.K2_SetTimerDelegate` (delegate `OnVictory`) (`self.VictoryTime`)))
  (set `self.VictoryTimerHandle` _returnvalue))

(event `OnVictory`
  (`self.StopSpawners`)
  (bind _asbp_third_person_character (cast `/Game/ThirdPerson/Blueprints/BP_ThirdPersonCharacter` (`GameplayStatics.GetPlayerPawn` 0)))
  (`/Game/ThirdPerson/Blueprints/BP_ThirdPersonCharacter.StopPlayer` _asbp_third_person_character)
  (`self.ShowResult` false)
  (bind _outactors (`GameplayStatics.GetAllActorsOfClass` "/Game/Enemy/BP_EnemyCharacter.BP_EnemyCharacter_C"))
  (for _array_element _outactors
    (`/Game/Enemy/BP_EnemyCharacter.StopEnemy` _array_element)))

(event `StopSpawners`
  (bind _outactors (`GameplayStatics.GetAllActorsOfClass` "/Game/Enemy/BP_Spawner.BP_Spawner_C"))
  (for _array_element _outactors
    (`/Game/Enemy/BP_Spawner.OnGameEnd` _array_element)))

(event `ShowResult`
  (params (IsVictory :type Boolean))
  (bind _returnvalue (`GameplayStatics.GetPlayerController` 0))
  (bind _asgs_survive_io (cast `/Game/SurviveIO/GS_SurviveIO` (`GameplayStatics.GetGameState`)))
  (bind _returnvalue_2 (`|CreateWidget` "/Game/UI/WBP_ResultScreen.WBP_ResultScreen_C" (`GameplayStatics.GetPlayerController` 0) IsVictory (`/Game/SurviveIO/GS_SurviveIO.IsHighscore` _asgs_survive_io)))
  (`UserWidget.AddToViewport` _returnvalue_2 0)
  (`WidgetBlueprintLibrary.SetInputMode_UIOnlyEx` _returnvalue null)
  (set `PlayerController.bShowMouseCursor` true _returnvalue))

(fn `SpawnDefaultPawnAtTransform`
  (params (NewPlayer :type "Controller Object Reference") (SpawnTransform :type "Transform Structure (by ref)"))
  (returns (ReturnValue :type "Pawn Object Reference"))
  (bind _returnvalue (`parent.SpawnDefaultPawnAtTransform` NewPlayer SpawnTransform))
  (add `/Game/Health/HealthComponent.OnDeath` (`self.GetComponentByClass` _returnvalue "/Game/Health/HealthComponent.HealthComponent_C") (`|CreateDelegate` :!event `OnPlayerDeath`))
  (return _returnvalue))

(fn `UserConstructionScript`)