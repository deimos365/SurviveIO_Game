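; Enemy pawn with a health component and world-space health bar that explodes when killed.
; Incoming damage feeds the HealthComponent, whose death event prints a debug message, unpossesses the controller, destroys the actor and spawns an explosion.
; BeginPlay binds the bar widget to the component.
; While moving, Tick turns the pawn toward the player at constant speed and the health bar toward the camera.
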(event `self.ReceiveAnyDamage`
  (params (Damage :type "Float (single-precision)") (DamageType :type "DamageType Object Reference") (InstigatedBy :type "Controller Object Reference") (DamageCauser :type "Actor Object Reference"))
  (`/Game/Health/HealthComponent.SetDamage` (`self.HealthComponent`) Damage))

(event `self.HealthComponent.OnDeath`
  (`KismetSystemLibrary.PrintString` "Enemy Dead" true true (struct :`G` 0.66 :`B` 1.0 :`A` 1.0) 5.0)
  (`self.StopEnemy`))

(event `StopEnemy`
  (`Controller.UnPossess` (`self.GetController`))
  (`self.K2_DestroyActor`)
  (`GameplayStatics.SpawnEmitterAtLocation` "/Game/StarterContent/Particles/P_Explosion.P_Explosion" (`self.K2_GetActorLocation`)))

(event `self.ReceiveTick`
  (params (DeltaSeconds :type "Float (single-precision)"))
  (if (> (`KismetMathLibrary.VSize` (`NavMovementComponent.GetVelocityForNavMovement` (`self.FloatingPawnMovement`))) 5.0)
    (`self.K2_SetActorRotation` (`KismetMathLibrary.RInterpTo_Constant` (`self.K2_GetActorRotation`) (`KismetMathLibrary.FindLookAtRotation` (`self.K2_GetActorLocation`) (`self.K2_GetActorLocation` (`GameplayStatics.GetPlayerCharacter` 0))) DeltaSeconds 300.0))
    (`SceneComponent.K2_SetWorldRotation` (`self.HealthBarWidget`) (`KismetMathLibrary.FindLookAtRotation` (`SceneComponent.K2_GetComponentLocation` (`self.HealthBarWidget`)) (`SceneComponent.K2_GetComponentLocation` (`PlayerCameraManager.TransformComponent` (`GameplayStatics.GetPlayerCameraManager` 0)))) false false)))

(event `self.ReceiveBeginPlay`
  (bind _aswbp_health_bar (cast `/Game/UI/WBP_HealthBar` (`WidgetComponent.GetUserWidgetObject` (`self.HealthBarWidget`))))
  (`/Game/UI/WBP_HealthBar.InitHealthBar` _aswbp_health_bar (`self.HealthComponent`)))

(fn `UserConstructionScript`)