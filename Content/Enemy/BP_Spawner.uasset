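; Enemy spawner actor that periodically spawns EnemyClass actors while the game is running.
; OnGameStart spawns one immediately and starts a looping timer at SpawnInterval, which OnGameEnd clears.
; Each spawn gets a random X/Y offset bounded by SpawnRadius at the spawner's height and always spawns, adjusting for collisions if possible.
; The spawned actor is then broadcast through the OnEnemySpawn dispatcher.
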(event Custom|SpawnEnemy
  (bind _returnvalue (Transformation|GetActorLocation))
  (bind _returnvalue_2 (Game|SpawnActorfromClass (Variables|Default|GetEnemyClass) (Math|Transform|MakeTransform (Math|Vector|MakeVector (+ (.x _returnvalue) (Math|Random|RandomFloatinRange (stale _result) (Variables|Default|GetSpawnRadius))) (+ (.y _returnvalue) (Math|Random|RandomFloatinRange (stale _result) (Variables|Default|GetSpawnRadius))) (.z _returnvalue)) "0, 0, 0" "1.000000,1.000000,1.000000") "AdjustIfPossibleButAlwaysSpawn" "MultiplyWithRoot" 0 0))
  (CallFunction|OnSpawn _returnvalue_2))

(event Custom|OnGameStart
  (bind _returnvalue (Utilities|Time|SetTimerbyEvent (delegate Custom|SpawnEnemy) (Variables|Default|GetSpawnInterval) true))
  (Variables|Default|SetTimer _returnvalue)
  (CallFunction|SpawnEnemy))

(event Custom|OnGameEnd
  (Utilities|Time|ClearandInvalidateTimerbyHandle (Variables|Default|GetTimer)))

(event Custom|OnSpawn
  (params (SpawnedActor :type Actor%20Object%20Reference))
  (Default|CallOnEnemySpawn SpawnedActor))

(event EventBeginPlay)

(fn ConstructionScript)